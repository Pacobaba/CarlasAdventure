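; Carla is a playable character Blueprint with Enhanced Input-style actions for movement, jumping and a spline-based camera.
; WS and AD move the character relative to controller yaw, and Space jumps.
; MouseLook accumulates a clamped distance fraction, placing the camera along a spline and pitching control rotation toward the mesh with yaw forced to zero.
; EsteInLimita, the construction script and overlap event are empty.
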(event Input|EnhancedActionEvents|EnhancedInputActionAD
  (params (ActionValue :type Float%20%28double-precision%29) (ElapsedSeconds :type Float%20%28double-precision%29) (TriggeredSeconds :type Float%20%28double-precision%29) (InputAction :type Input%20Action%20Object%20Reference :default "/Game/BluePrints/GameLogic/Controls/AD.AD"))
  (Pawn|Input|AddMovementInput (Math|Vector|GetRightVector (Math|Rotator|MakeRotator 0.0 0.0 (.yaw (Pawn|GetControlRotation (Pawn|GetController) :!class /Script/Engine.Controller)))) ActionValue false))

(event Input|EnhancedActionEvents|EnhancedInputActionSpace
  (params (ActionValue :type Boolean) (ElapsedSeconds :type Float%20%28double-precision%29) (TriggeredSeconds :type Float%20%28double-precision%29) (InputAction :type Input%20Action%20Object%20Reference :default "/Game/BluePrints/GameLogic/Controls/Space.Space"))
  (Character|Jump))

(event Input|EnhancedActionEvents|EnhancedInputActionMouseLook
  (params (ActionValue :type Float%20%28double-precision%29) (ElapsedSeconds :type Float%20%28double-precision%29) (TriggeredSeconds :type Float%20%28double-precision%29) (InputAction :type Input%20Action%20Object%20Reference :default "/Game/BluePrints/GameLogic/Controls/MouseLook.MouseLook"))
  (bind _output_get (Variables|Default|SetdistantaPeSpline (Math|Float|Clamp(Float) (+ (/ ActionValue 3e+01) (Variables|Default|GetdistantaPeSpline)))))
  (Transformation|SetWorldLocationAndRotation (Variables|Default|GetCamera) (Spline|GetLocationatDistanceAlongSpline (Variables|Default|GetSpline) (Math|Float|Lerp 0.0 (Spline|GetSplineLength (Variables|Default|GetSpline)) _output_get) "World") "0, 0, 0" false false)
  (Pawn|SetControlRotation (Pawn|GetController) (Math|Rotator|MakeRotator 0.0 (.pitch (Math|Rotator|FindLookatRotation (Transformation|GetWorldLocation (Variables|Default|GetCamera)) (Transformation|GetWorldLocation (Variables|Character|GetMesh)))) 0.0)))

(event Input|EnhancedActionEvents|EnhancedInputActionWS
  (params (ActionValue :type Float%20%28double-precision%29) (ElapsedSeconds :type Float%20%28double-precision%29) (TriggeredSeconds :type Float%20%28double-precision%29) (InputAction :type Input%20Action%20Object%20Reference :default "/Game/BluePrints/GameLogic/Controls/WS.WS"))
  (Pawn|Input|AddMovementInput (Math|Vector|GetForwardVector (Math|Rotator|MakeRotator 0.0 0.0 (.yaw (Pawn|GetControlRotation (Pawn|GetController) :!class /Script/Engine.Controller)))) ActionValue false))

(event EventBeginPlay
  (Input|EnableInput (Game|GetPlayerController 0)))

(event Collision|EventActorBeginOverlap
  (params (OtherActor :type Actor%20Object%20Reference)))

(fn ConstructionScript)

(fn EsteinLimita)